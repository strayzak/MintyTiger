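; Pushable interactive actor that, on interaction, snaps a character to a push position and starts a push through its Push_Component.
; Push transforms appear as construction-script arrows; the closest-in-range search exists but is disconnected from its function entry.
; Before teleporting, HandleInteraction checks standing room and walkable floor with a capsule trace, and obstructions with a line trace.
; Debug drawing and printed failure reasons expose each check.
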(event `/Game/Interactives/Interact_Interface/Interact_Interface.OnInteracted`
  (params (Player :type "/Game/Characters/Fairy_RootBone/BP_Fairy Object Reference"))
  (`self.HandleInteraction` Player))

(fn `FindClosestPushTransformIndex`
  (params (CharacterLocation :type "Vector2D Structure") (PushRange :type "Float (double-precision)"))
  (returns (BestIndex :type Integer))
  (locals (CurrentTransformIndex :type Integer) (CurrentDistanceSq :type "Float (double-precision)" :default 0.0) (ClosestTransformIndex :type Integer :default -1) (ClosestDistanceSq :type "Float (double-precision)")))

(fn `HandleInteraction`
  (params (Character :type "Character Object Reference"))
  (locals (PushComponent :type "/Game/Interactives/Pushable/Push_Component Object Reference") (CharacterNewTransform :type "Transform Structure"))
  (bind _characternewtransform_location (`KismetMathLibrary.BreakTransform` (`local.CharacterNewTransform`)))
  (bind _characternewtransform_location_2 (`KismetMathLibrary.BreakTransform` (`local.CharacterNewTransform`)))
  (bind _capsulecomponent (`Character.CapsuleComponent` (`local.Character`)))
  (`/Engine/EditorBlueprintResources/StandardMacros.IsValid` Character
    (:`Is Valid`
      (bind _output_get (set `local.PushComponent` (`self.GetComponentByClass` Character "/Game/Interactives/Pushable/Push_Component.Push_Component_C")))
      (`/Engine/EditorBlueprintResources/StandardMacros.IsValid` _output_get
        (:`Is Valid`
          (bind _bestindex (`self.FindClosestPushTransformIndex` (`KismetMathLibrary.Conv_VectorToVector2D` (`self.K2_GetActorLocation` (`local.Character`))) (`/Game/Interactives/Pushable/Push_Component.PushRange` (`local.PushComponent`))))
          (if (>= _bestindex 0)
            (bind (_returnvalue_location _returnvalue_rotation _returnvalue_scale) (`KismetMathLibrary.BreakTransform` (`KismetMathLibrary.ComposeTransforms` (`|GetArrayItem` (`self.PushTransforms`) _bestindex) (`self.GetTransform`))))
            (bind _output_get_2 (set `local.CharacterNewTransform` (`KismetMathLibrary.MakeTransform` (+ _returnvalue_location (`KismetMathLibrary.MakeVector` 0.0 0.0 (`CapsuleComponent.GetScaledCapsuleHalfHeight` (`Character.CapsuleComponent` (`local.Character`))))) _returnvalue_rotation _returnvalue_scale)))
            (`KismetSystemLibrary.DrawDebugSphere` (.location _output_get_2) 20.0 12 (struct :`R` 1.0 :`A` 1.0) 2.0 1.0)
            (bind _outhit (`KismetSystemLibrary.CapsuleTraceSingle` :`Start` (+ _characternewtransform_location_2 (0.0 0.0 70.0)) :`End` (- _characternewtransform_location_2 (0.0 0.0 100.0)) :`Radius` (`CapsuleComponent.GetScaledCapsuleRadius` _capsulecomponent) :`HalfHeight` (`CapsuleComponent.GetScaledCapsuleHalfHeight` _capsulecomponent) :`TraceChannel` "TraceTypeQuery1" :`DrawDebugType` "ForDuration" :`DrawTime` 2.0))
            (bind (_bblockinghit _binitialoverlap _time _distance _location _impactpoint _normal _impactnormal) (`GameplayStatics.BreakHitResult` _outhit))
            (if (not _binitialoverlap)
              (if (< (`CharacterMovementComponent.K2_GetWalkableFloorZ` (`Character.CharacterMovement` (`local.Character`))) (.z _impactnormal))
                (bind (_outhit_2 _returnvalue) (`KismetSystemLibrary.LineTraceSingle` (`self.K2_GetActorLocation`) _characternewtransform_location "TraceTypeQuery1" false (`|MakeArray` (`local.Character`) null :!type "Actor Object Reference") "ForDuration" true (struct :`R` 1.0 :`A` 1.0) (struct :`G` 1.0 :`A` 1.0) 2.0))
                (`KismetSystemLibrary.PrintString` (`KismetSystemLibrary.GetDisplayName` (`.HitActor` (`GameplayStatics.BreakHitResult` _outhit_2))))
                (if (not _returnvalue)
                  (`self.K2_SetActorTransform` (`local.Character`) (`local.CharacterNewTransform`) false true)
                  (`/Game/Interactives/Pushable/Push_Component.BeginPush` (`local.PushComponent`) self)
                  (else
                    (`self.PushFailedInfo` "Wall in between character and object")))
                (else
                  (`self.PushFailedInfo` "Floor not walkable")))
              (else
                (`self.PushFailedInfo` "No room to stand")))
            (else
              (`self.PushFailedInfo` "No push transform found"))))
        (:`Is Not Valid`
          (`self.PushFailedInfo` "Character does not have push component"))))
    (:`Is Not Valid`
      (`self.PushFailedInfo` "Character is invalid"))))

(fn `UserConstructionScript`
  (for _array_element (`self.PushTransforms`)
    (`AddComponent|NODE_AddArrowComponent-0` :`RelativeTransform` _array_element)))